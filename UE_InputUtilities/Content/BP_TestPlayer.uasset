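; BP_TestPlayer is a test player Blueprint that exercises Enhanced Input actions and a pause menu.
; On BeginPlay it adds a test mapping context, and its jump and interact actions only print debug messages.
; An Escape debug key, ignored while a key remap is in progress, toggles a paused flag that adds or removes BP_PauseMenu and switches input mode and cursor visibility.
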(event Input|EnhancedActionEvents|EnhancedInputActionIA_Test_Jump
  (params (ActionValue :type Boolean) (ElapsedSeconds :type Float%20%28double-precision%29) (TriggeredSeconds :type Float%20%28double-precision%29) (InputAction :type Input%20Action%20Object%20Reference :default "/Game/IA_Test_Jump.IA_Test_Jump"))
  (:Started
    (Development|PrintString "JumpPressed")))

(event Input|EnhancedActionEvents|EnhancedInputActionIA_Test_Interact
  (params (ActionValue :type Boolean) (ElapsedSeconds :type Float%20%28double-precision%29) (TriggeredSeconds :type Float%20%28double-precision%29) (InputAction :type Input%20Action%20Object%20Reference :default "/Game/IA_Test_Interact.IA_Test_Interact"))
  (:Started
    (Development|PrintString "Interact Pressed")))

(event EventBeginPlay
  (Input|AddMappingContext (PlayerController|LocalPlayerSubsystems|GetEnhancedInputLocalPlayerSubsystem (Game|GetPlayerController 0)) "/Game/TestMappingContext.TestMappingContext" 0 "(bIgnoreAllPressedKeysUntilRelease=True,bForceImmediately=False)"))

(event Input|KeyboardEvents|DebugKeyEscape
  (params (Key :type Key%20Structure :default "None") (ActionValue :type Input%20Action%20Value%20Structure))
  (bind _returnvalue (Game|GetPlayerController 0))
  (bind _returnvalue_2 (Game|GetPlayerController 0))
  (:Pressed
    (if (not (Variables|/Script/InputUtilities.InputUtilitySubsystem|GetbInProcessOfRemappingKey (Subsystems|GetInputUtilitySubsystem)))
      (Variables|Default|SetPaused (not (Variables|Default|GetPaused)))
      (if (Variables|Default|GetPaused)
        (Utilities|FlowControl|Sequence
          (:then_0
            (Input|SetInputModeGameandUI _returnvalue_2 0 "DoNotLock" true false)
            (Variables|/Script/Engine.PlayerController|SetbShowMouseCursor _returnvalue_2 true))
          (:then_1
            (bind _returnvalue_3 (UserInterface|CreateWidget "/Game/BP_PauseMenu.BP_PauseMenu_C"))
            (Variables|Default|SetPauseMenu _returnvalue_3)
            (UserInterface|Viewport|AddtoViewport _returnvalue_3 0)))
        (else
          (Utilities|FlowControl|Sequence
            (:then_0
              (Widget|RemovefromParent (Variables|Default|GetPauseMenu)))
            (:then_1
              (Input|SetInputModeGameOnly _returnvalue false)
              (Variables|/Script/Engine.PlayerController|SetbShowMouseCursor _returnvalue false))))))))

(fn ConstructionScript)